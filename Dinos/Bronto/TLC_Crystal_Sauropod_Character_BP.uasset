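; Character Blueprint for the Crystal Sauropod dino, adding a server-configurable incoming damage multiplier on top of its parent's behavior.
; On BeginPlay the server reads CrystalDinoDamage from the SauropodPack ini section through ShooterGameMode and applies it as ExtraReceiveDamageMultiplier.
; Because the value is floored before the check, any setting below 1 falls back to a built-in damage-reduction default.
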(event `self.ReceiveBeginPlay`
  (`parent.ReceiveBeginPlay`)
  (`/Engine/EditorBlueprintResources/ActorMacros.Switch Has Authority`
    (:`Authority`
      (bind _asshootergamemode (cast `ShooterGameMode` (`GameplayStatics.GetGameMode`)))
      (bind _returnvalue (`ShooterGameMode.GetFloatOptionIni` _asshootergamemode "SauropodPack" "CrystalDinoDamage"))
      (if (<= (`KismetMathLibrary.FFloor` _returnvalue) 0)
        (set `self.ExtraReceiveDamageMultiplier` 0.8)
        (else
          (set `self.ExtraReceiveDamageMultiplier` _returnvalue))))))

(fn `UserConstructionScript`
  (`parent.UserConstructionScript`))