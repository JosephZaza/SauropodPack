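; Seismo dino character with a health-gated custom taming method and a fuel-consuming factory saddle.
; On authority, BeginPlay can override the taming threshold from the SauropodPack INI; Tick, throttled by a Delay, allows torpor only below that health or once tamed.
; When tamed, Tick also burns saddle fuel from inventory at timed intervals on standalone or server, gated by an IsEquipped comparison.
; HasFactorySaddle always returns true, as does AllowWakingTame.
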(event EventTick
  (params (DeltaSeconds :type Float%20%28single-precision%29))
  (Utilities|FlowControl|Sequence
    (:then_0
      (if (Variables|Default|GetUseCustomTamingMethod)
        (Utilities|FlowControl|Delay 1.0)
        (if (Class|PrimalDinoCharacter|BPIsTamed)
          (Variables|Default|SetbCanBeTorpid true :!label _label)
          (elif (>= (Class|PrimalCharacter|GetHealthPercentage) (Variables|Default|GetPercentToTame))
            (Variables|Default|SetbCanBeTorpid false)
            (elif (not (Variables|Default|GetbCanBeTorpid))
              (Utilities|FlowControl|Sequence
                (:then_0
                  (goto _label))))))))
    (:then_1
      (if (Class|PrimalDinoCharacter|BPIsTamed)
        (if (Math|Boolean|Equal(Boolean) (stale _isequiped) (Variables|Default|GetIsEquipped))
          (if (> (stale _quantity) 0)
            (CallFunction|ConsumeGas)))))))

(event EventBeginPlay
  (|CallParentFunction)
  (Networking|SwitchHasAuthority
    (:Authority
      (bind _asshootergamemode (Utilities|Casting|CastToShooterGameMode (Game|GetGameMode)))
      (bind _returnvalue (Class|ShooterGameMode|GetFloatOptionIni _asshootergamemode "SauropodPack" "SeismoHealthToTame"))
      (if (< _returnvalue 0.0)
        (Variables|Default|SetPercentToTame (Variables|Default|GetPercentToTame))
        (else
          (Variables|Default|SetPercentToTame _returnvalue))))))

(fn ConstructionScript
  (|CallParentFunction))

(fn AllowWakingTame
  (params (ForPC :type Player%20Controller%20Object%20Reference))
  (return true))

(fn ConsumeGas
  (Utilities|FlowControl|Sequence
    (:then_0
      (Class|KismetSystemLibrary|SwitchNetworkMode
        (:Standalone
          _)
        (:DedicatedServer
          _)
        (:ListenServer
          _))
      (if (Class|VictoryCore|IsTimeSinceNetwork (Class|Actor|GetWorld) (Variables|Default|GetLastConsumeFuelTime) (Variables|Default|GetFuelConsumeFrequency) true)
        (Variables|Default|SetLastConsumeFuelTime (Class|VictoryCore|GetNetworkTimeinSeconds))
        (CallFunction|ConsumeItem (Variables|Default|GetSaddleFuelItem))))))

(fn ConsumeItem
  (params (Item :type Primal%20Item%20Resource%20Gasoline%20Class%20Reference))
  (Class|PrimalInventoryComponent|BPIncrementItemTemplateQuantity (Variables|Default|GetMyInventoryComponent) Item -1 true false false false true false 0 true))

(fn HasGas
  (bind _returnvalue (Class|PrimalInventoryComponent|GetItemTemplateQuantity (Variables|Default|GetMyInventoryComponent) (Variables|Default|GetSaddleFuelItem) 0 true false false false))
  (return (> _returnvalue 0) _returnvalue))

(fn HasFactorySaddle
  (Class|PrimalItem|BlueprintEquipped (Variables|Default|GetFactorySaddle) false)
  (return true))