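; Crystal Seismo sauropod dino character with a health-gated taming rule and waking taming allowed.
; On authority, begin-play events read SauropodPack INI options for a health-to-tame threshold and extra received-damage multiplier, with fallbacks.
; With custom taming enabled, a delayed Tick check blocks torpor while an untamed Seismo's health is at or above PercentToTame, allowing it once lower or tamed.
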(event `ReceiveBeginPlay_Copy`
  (`parent.ReceiveBeginPlay`)
  (`/Engine/EditorBlueprintResources/ActorMacros.Switch Has Authority`
    (:`Authority`
      (bind _asshootergamemode (cast `ShooterGameMode` (`GameplayStatics.GetGameMode`)))
      (bind _returnvalue (`ShooterGameMode.GetFloatOptionIni` _asshootergamemode "SauropodPack" "CrystalDinoDamage"))
      (if (<= (`KismetMathLibrary.FFloor` _returnvalue) 0)
        (set `self.ExtraReceiveDamageMultiplier` 0.8)
        (else
          (set `self.ExtraReceiveDamageMultiplier` _returnvalue))))))

(event `self.ReceiveBeginPlay`
  (`parent.ReceiveBeginPlay`)
  (`/Engine/EditorBlueprintResources/ActorMacros.Switch Has Authority`
    (:`Authority`
      (bind _asshootergamemode (cast `ShooterGameMode` (`GameplayStatics.GetGameMode`)))
      (bind _returnvalue (`ShooterGameMode.GetFloatOptionIni` _asshootergamemode "SauropodPack" "SeismoHealthToTame"))
      (if (<= _returnvalue 0.0)
        (set `self.PercentToTame_0` (`self.PercentToTame`))
        (else
          (set `self.PercentToTame_0` _returnvalue))))))

(event `self.ReceiveTick`
  (params (DeltaSeconds :type "Float (single-precision)"))
  (if (`self.UseCustomTamingMethod`)
    (`KismetSystemLibrary.Delay` 1.0)
    (if (`self.BPIsTamed`)
      (set `self.bCanBeTorpid` true :!label _label)
      (elif (>= (`self.GetHealthPercentage`) (`self.PercentToTame`))
        (set `self.bCanBeTorpid` false)
        (elif (not (`self.bCanBeTorpid`))
          (`|ExecutionSequence`
            (:`then_0`
              (goto _label))))))))

(fn `AllowWakingTame`
  (params (ForPC :type "PlayerController Object Reference"))
  (returns (ReturnValue :type Boolean))
  (return true))

(fn `NewFunction_0`)

(fn `UserConstructionScript`
  (`parent.UserConstructionScript`))