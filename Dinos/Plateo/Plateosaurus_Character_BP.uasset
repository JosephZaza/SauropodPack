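; Character Blueprint for the Plateosaurus dino, overriding rider attack, interaction and jump hooks.
; The rider attack check allows the primary attack only when submerged and turns the third input into a different attack when not submerged.
; Living tamed dinos offer same-team players a colored use entry, hard-wired disabled with no handler here.
; Many conditions and jump values are constants, leaving several overrides as stubs or parent pass-throughs.
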(fn ConstructionScript
  (|CallParentFunction))

(fn BlueprintCanRiderAttack
  (params (AttackIndex :type Integer))
  (bind _returnvalue (Class|PrimalCharacter|IsSubmerged false false false false))
  (bind _returnvalue_2 (not false))
  (bind _returnvalue_3 (not _returnvalue))
  (LocalVariables|SetretVal false)
  (Utilities|FlowControl|Sequence
    (:then_0
      (switch int AttackIndex
        (:0
          (if (or false _returnvalue)
            (LocalVariables|SetretVal _returnvalue_2 :!label _label)
            (elif _returnvalue_2
              _)))
        (:1
          (bind _returnvalue_4 (Class|PrimalDinoCharacter|IsAttacking))
          (if (and _returnvalue_3 (not _returnvalue_4))
            _))
        (:2
          (if _returnvalue_3
            (if true
              (Class|PrimalDinoCharacter|DoAttack 3 true false)
              (else
                (goto _label)))))))
    (:then_1
      (return (LocalVariables|GetretVal)))))

(fn ReceiveAnyDamage
  (params (Damage :type Float%20%28single-precision%29) (DamageType :type Damage%20Type%20Object%20Reference) (InstigatedBy :type Controller%20Object%20Reference) (DamageCauser :type Actor%20Object%20Reference))
  (|CallParentFunction Damage DamageType InstigatedBy DamageCauser)
  (if (and (not false) (not (Variables|Default|GetbHasRider)))
    _))

(fn BPNotifySetRider
  (params (RiderSetting :type Shooter%20Character%20Object%20Reference))
  (|CallParentFunction RiderSetting))

(fn BPGetMultiUseEntries
  (params (ForPC :type Player%20Controller%20Object%20Reference) (MultiUseEntries :type Array%20of%20Multi%20Use%20Entry%20Structures))
  (if (Math|Boolean|ANDBoolean (Class|PrimalDinoCharacter|BPIsTamed) (== (Variables|/Script/Engine.Actor|GetTargetingTeam ForPC) (Variables|Default|GetTargetingTeam)) (Class|PrimalCharacter|IsAlive))
    (Utilities|Array|Add MultiUseEntries (Utilities|Struct|MakeMultiUseEntry 0 "" 3000 20 false (or (not false) (not (Class|PrimalCharacter|BPIsConscious))) false false false false false false false true false false false false 0 "(B=175,G=175,R=175,A=255)" (Math|Conversions|ToColor(LinearColor) "(R=1.000000,G=0.696103,B=0.195000,A=1.000000)"))))
  (return MultiUseEntries))

(fn BPUnstasis
  (|CallParentFunction))

(fn BlueprintAnimNotifyCustomEvent
  (params (CustomEventName :type Name :default "None") (MeshComp :type Skeletal%20Mesh%20Component%20Object%20Reference) (Animation :type Anim%20Sequence%20Base%20Object%20Reference) (AnimNotifyObject :type Anim%20Notify%20Object%20Reference)))

(fn BPTimerServer)

(fn BPGetAddForwardVelocityonJump
  (return (* (Math|Float|SelectFloat 0.0 0.0 false) (Math|Float|SelectFloat 1.0 (Math|Float|SelectFloat 0.0 0.0 (Class|PrimalCharacter|IsMoving)) (Variables|Default|GetbWantsToRun)))))

(fn CanJumpInternal
  (return (and (>= (Class|VictoryCore|TimeSince (Class|Actor|GetWorld) 0.0) 0.0) (|CallParentFunction))))

(fn OnJumped
  (|CallParentFunction))