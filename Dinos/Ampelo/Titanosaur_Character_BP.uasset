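; Titanosaur character Blueprint for a giant raid dino with special knockout and taming rules.
; Head hits from raid-torpor damage add torpor only while it walks unobstructed and keeps moving, with a distance-based cap against trapping, and temporarily let it target neutral structures.
; Wild AI is forced to flee targets far above or below.
; Without raid-dino feeding, XP and auto-eating are disabled and randomized timers tick tamed status manually on the server.
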(event Custom|ForceTamedTick
  (bind _returnvalue (Utilities|Time|GetGameTimeinSeconds))
  (if (and (Class|PrimalDinoCharacter|BPIsTamed) (Class|PrimalCharacter|IsAlive))
    (if (> (Math|Conversions|ToFloat(Integer) (Variables|Default|GetLastCharacterStatusTickTime)) 0.0)
      (Class|PrimalCharacterStatusComponent|TickStatus (Variables|Default|GetMyCharacterStatusComponent) (Math|Conversions|ToFloat(Integer) (- _returnvalue (Variables|Default|GetLastCharacterStatusTickTime))) true))
    (Variables|Default|SetLastCharacterStatusTickTime _returnvalue))
  (Utilities|Time|SetTimerbyFunctionName 0 "ForceTamedTick" (Math|Random|RandomFloatinRange 1.0 2.0)))

(event Custom|ClearTorporHit
  (Variables|Default|SetbWildAllowTargetingNeutralStructures false))

(event Custom|TorporHit
  (if (and (Networking|IsServer) (Class|PrimalCharacter|BPIsConscious))
    (Class|PrimalCharacter|PlayAnimEx "/Game/PrimalEarth/Dinos/Titanosaur/Animations/Titanosaur-Hurt-Rit_Montage.Titanosaur-Hurt-Rit_Montage" 1.0 "None" true true true true false 0.0 0.0)))

(event EventTick
  (params (DeltaSeconds :type Float%20%28single-precision%29))
  (bind _returnvalue (Transformation|GetActorLocation))
  (bind _z (Math|Vector|BreakVector _returnvalue))
  (if (and (Networking|IsServer) (not (Class|PrimalDinoCharacter|BPIsTamed)))
    (bind _asprimaldinoaicontroller (Utilities|Casting|CastToPrimalDinoAIController (Pawn|GetController)))
    (bind _returnvalue_2 (Class|PrimalDinoAIController|GetTarget _asprimaldinoaicontroller))
    (if (Utilities|IsValid _returnvalue_2)
      (if (> (.Z (Math|Vector|BreakVector (Transformation|GetActorLocation _returnvalue_2))) (+ _z 1.8e+03))
        (Variables|/Script/ShooterGame.PrimalDinoAIController|SetLastForcedFleeTime _asprimaldinoaicontroller (Utilities|Time|GetGameTimeinSeconds) :!label _label)
        (elif (> (- _z 3.2e+03) (.Z (Math|Vector|BreakVector (Transformation|GetActorLocation _returnvalue_2))))
          (goto _label))))))

(fn ConstructionScript
  (|CallParentFunction))

(fn BPAdjustDamage
  (params (IncomingDamage :type Float%20%28single-precision%29) (TheDamageEvent :type Damage%20Event%20Structure) (EventInstigator :type Controller%20Object%20Reference) (DamageCauser :type Actor%20Object%20Reference) (bIsPointDamage :type Boolean) (PointHitInfo :type Hit%20Result%20Structure))
  (if bIsPointDamage
    (if (>= (Utilities|Array|FindItem (Variables|Default|GetTorporHeadBoneNames) (.HitBoneName (Collision|BreakHitResult PointHitInfo))) 0)
      (bind _returnvalue (Class|VictoryCore|GetClassDefaultObject (.DamageTypeClass (Utilities|Struct|BreakDamageEvent TheDamageEvent))))
      (bind _asshooterdamagetypebp_base_c (Utilities|Casting|CastToShooterDamageTypeBP_Base _returnvalue)
        (:then
          (if (and (Variables|/Game/PrimalEarth/CoreBlueprints/DamageTypes/ShooterDamageTypeBP_Base.ShooterDamageTypeBP_Base_C|GetbCauseRaidTorpor _asshooterdamagetypebp_base_c) (Utilities|Enum|Equal(Enum) (Variables|/Script/Engine.CharacterMovementComponent|GetMovementMode (Variables|Character|GetCharacterMovement)) "MOVE_Walking"))
            (bind _bhasmoved (CallFunction|HasMovedRecently))
            (if _bhasmoved
              (if (not (CallFunction|IsHeadObstructed))
                (bind _outvaliddistancetravel (CallFunction|CheckTorporDistanceTravel (* IncomingDamage (Variables|/Game/PrimalEarth/CoreBlueprints/DamageTypes/ShooterDamageTypeBP_Base.ShooterDamageTypeBP_Base_C|GetRaidTorporDamageMultiplier _asshooterdamagetypebp_base_c))))
                (if _outvaliddistancetravel
                  (bind _asdinocharacterstatuscomponent_bp_titanosaur_c (Utilities|Casting|CastToDinoCharacterStatusComponent_BP_Titanosaur (Variables|Default|GetMyCharacterStatusComponent)))
                  (Variables|/Game/PrimalEarth/CoreBlueprints/DinoCharacterStatusComponent_BP_Titanosaur.DinoCharacterStatusComponent_BP_Titanosaur_C|SetbAllowTorpidityIncrease _asdinocharacterstatuscomponent_bp_titanosaur_c true)
                  (Class|PrimalCharacterStatusComponent|ModifyCurrentStatusValue _asdinocharacterstatuscomponent_bp_titanosaur_c "Torpidity" (* IncomingDamage (Variables|/Game/PrimalEarth/CoreBlueprints/DamageTypes/ShooterDamageTypeBP_Base.ShooterDamageTypeBP_Base_C|GetRaidTorporDamageMultiplier _asshooterdamagetypebp_base_c)) false false true false "/Script/Engine.DamageType" false false)
                  (Variables|/Game/PrimalEarth/CoreBlueprints/DinoCharacterStatusComponent_BP_Titanosaur.DinoCharacterStatusComponent_BP_Titanosaur_C|SetbAllowTorpidityIncrease _asdinocharacterstatuscomponent_bp_titanosaur_c false)
                  (Variables|Default|SetbWildAllowTargetingNeutralStructures true)
                  (Utilities|Time|SetTimerbyFunctionName 0 "TorporHit" 0.05)
                  (Utilities|Time|SetTimerbyFunctionName 0 "ClearTorporHit" 6e+01))))))
        (:CastFailed
          _))))
  (return IncomingDamage))

(fn ReceiveBeginPlay
  (if (Networking|IsServer)
    (bind _asshootergamestate (Utilities|Casting|CastToShooterGameState (Game|GetGameState)))
    (if (not (Variables|/Script/ShooterGame.ShooterGameState|GetbAllowRaidDinoFeeding _asshootergamestate))
      (Utilities|Time|SetTimerbyFunctionName 0 "ForceTamedTick" (Math|Random|RandomFloatinRange 1.0 2.0))
      (Variables|Default|SetbForceNoCharacterStatusComponentTick true))))

(fn BPPostInitializeComponents
  (bind _mycharacterstatuscomponent (Variables|Default|GetMyCharacterStatusComponent))
  (bind _returnvalue (Class|VictoryCore|IsGameWorld (Class|Actor|GetWorld)))
  (if _returnvalue
    (bind _asshootergamestate (Utilities|Casting|CastToShooterGameState (Game|GetGameState)))
    (if (Variables|/Script/ShooterGame.ShooterGameState|GetbAllowRaidDinoFeeding _asshootergamestate)
      (Class|PrimalCharacterStatusComponent|BPSetRecoveryRateStatusValue _mycharacterstatuscomponent "Torpidity" -0.1)
      (else
        (Variables|Default|SetbAllowDinoAutoConsumeInventoryFood false)
        (Variables|/Script/ShooterGame.PrimalCharacterStatusComponent|SetbNeverAllowXP _mycharacterstatuscomponent true)))))

(fn GiveKillExperience
  (LocalVariables|SetretVal true)
  (if (Class|PrimalDinoCharacter|BPIsTamed)
    (LocalVariables|SetretVal false))
  (return (LocalVariables|GetretVal)))

(fn HasMovedRecently
  (bind _returnvalue (Utilities|Time|GetGameTimeinSeconds))
  (bind _returnvalue_2 (Transformation|GetActorLocation))
  (if (and (< (Math|Conversions|ToFloat(Integer) (- _returnvalue (Variables|Default|GetLastHasMovedRecentlyTime))) 5.0) (Variables|Default|GetLastHasMovedRecentlyRetVal))
    _
    (elif (> (Math|Vector|VectorLength (- _returnvalue_2 (Variables|Default|GetLastHasMovedRecentlyLocation))) 2e+02)
      (Variables|Default|SetLastHasMovedRecentlyRetVal true)
      (Variables|Default|SetLastHasMovedRecentlyLocation _returnvalue_2)
      (Variables|Default|SetLastHasMovedRecentlyTime _returnvalue)
      (else
        (Variables|Default|SetLastHasMovedRecentlyRetVal false))))
  (return (Variables|Default|GetLastHasMovedRecentlyRetVal)))

(fn IsHeadObstructed
  (bind _mesh (Variables|Character|GetMesh))
  (bind _returnvalue (Collision|LineTraceByChannel (Transformation|GetSocketLocation _mesh "NeckTraceStart") (Transformation|GetSocketLocation _mesh "NeckTraceEnd") "ECC_GameTraceChannel11" false 0 "None"))
  (return _returnvalue))

(fn CheckTorporDistanceTravel
  (params (torporIn :type Float%20%28single-precision%29))
  (bind _returnvalue (Transformation|GetActorLocation))
  (LocalVariables|SettheRetVal true)
  (if (== (Math|Vector|VectorLength (Variables|Default|GetTorporStartedDamageLocation)) 0.0)
    (Variables|Default|SetTorporStartedDamageLocation _returnvalue)
    (elif (< (Variables|Default|GetTorporDamageLocationCache) (Variables|Default|GetMaxTorporDamageForLocation))
      (Variables|Default|SetTorporDamageLocationCache (+ (Variables|Default|GetTorporDamageLocationCache) torporIn))
      (elif (> (Math|Vector|VectorLength (- _returnvalue (Variables|Default|GetTorporStartedDamageLocation))) (Variables|Default|GetTorporDamageLocationDistanceReset))
        (Variables|Default|SetTorporDamageLocationCache 0.0)
        (Variables|Default|SetTorporStartedDamageLocation _returnvalue)
        (else
          (LocalVariables|SettheRetVal false)))))
  (return (LocalVariables|GettheRetVal)))

(fn BPSetupTamed
  (params (bWasJustTamed :type Boolean))
  (bind _attackinfos (Variables|Default|GetAttackInfos))
  (bind _mycharacterstatuscomponent (Variables|Default|GetMyCharacterStatusComponent))
  (bind _item (Utilities|Array|Get(acopy) _attackinfos))
  (Utilities|FlowControl|Sequence
    (:then_0
      (Class|PrimalCharacterStatusComponent|BPSetRecoveryRateStatusValue _mycharacterstatuscomponent "Health" 4.0)
      (Utilities|Struct|SetmembersinDinoAttackInfo _item false false false false false false false false false false false false false false false false false false 0.0 (* (.MeleeSwingRadius (Utilities|Struct|BreakDinoAttackInfo _item)) 0.9) 1.0))
    (:then_1
      (bind _asshootergamestate (Utilities|Casting|CastToShooterGameState (Game|GetGameState)))
      (Utilities|FlowControl|Sequence
        (:then_0
          (if (Variables|/Script/ShooterGame.ShooterGameState|GetbServerPVE _asshootergamestate)
            (Variables|/Script/ShooterGame.PrimalCharacterStatusComponent|SetBaseFoodConsumptionRate _mycharacterstatuscomponent -0.034)))
        (:then_1
          (if (not (Variables|/Script/ShooterGame.ShooterGameState|GetbAllowRaidDinoFeeding _asshootergamestate))
            (Variables|Default|SetbAllowDinoAutoConsumeInventoryFood false)))))))

(fn BlueprintCanRiderAttack
  (params (AttackIndex :type Integer))
  (bind _returnvalue (CallFunction|BlueprintCanAttack AttackIndex 0.0 0.0))
  (return _returnvalue))

(fn BlueprintCanAttack
  (params (AttackIndex :type Integer) (distance :type Float%20%28single-precision%29) (attackRangeOffset :type Float%20%28single-precision%29) (OtherTarget :type Actor%20Object%20Reference))
  (bind _swimmingattackindex (Variables|Default|GetSwimmingAttackIndex))
  (LocalVariables|SetretVal false)
  (Utilities|FlowControl|Sequence
    (:then_0
      (switch int AttackIndex
        (:0
          (if (Class|PrimalCharacter|IsSubmerged false false false false)
            (bind _returnvalue (Class|PrimalDinoCharacter|CanAttack _swimmingattackindex))
            (if _returnvalue
              (Class|PrimalDinoCharacter|DoAttack _swimmingattackindex true false)
              (LocalVariables|SetretVal true))
            (else
              (LocalVariables|SetretVal (Utilities|Enum|Equal(Enum) (Variables|/Script/Engine.CharacterMovementComponent|GetMovementMode (Variables|Character|GetCharacterMovement)) "MOVE_Walking")))))
        (:2
          (LocalVariables|SetretVal (not (Variables|Default|GetbHasRider))))))
    (:then_1
      (return (LocalVariables|GetretVal)))))

(fn GetSocketforMeleeTraceforHitBlockers
  (params (AttackIndex :type Integer))
  (return "buffsocketcenterdynamic"))