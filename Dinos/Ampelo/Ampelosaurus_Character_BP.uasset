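; Ampelosaurus dino character Blueprint, a sauropod whose extra running speed boosts melee damage and fills a HUD progress bar.
; On BeginPlay the server sets its received-damage multiplier from the SauropodPack INI option, with a fallback default.
; Raid-torpor hits to head bones while walking briefly unlock the status component to add torpidity.
; Those hits also trigger a delayed startle montage and temporarily let wild ones target neutral structures.
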(event Custom|ClearTorporHit
  (Variables|Default|SetbWildAllowTargetingNeutralStructures false))

(event Custom|TorporHit
  (if (and (Networking|IsServer) (Class|PrimalCharacter|BPIsConscious))
    (Class|PrimalCharacter|PlayAnimEx "/Game/Mods/SauroPack/Dinos/Ampelo/Animations/Diplodocus-Startled-Rit_Montage_Copy_Copy_Copy.Diplodocus-Startled-Rit_Montage_Copy_Copy_Copy" 1.0 "None" true true false true false 0.0 0.0)))

(event EventBeginPlay
  (|CallParentFunction)
  (Networking|SwitchHasAuthority
    (:Authority
      (bind _asshootergamemode (Utilities|Casting|CastToShooterGameMode (Game|GetGameMode)))
      (bind _returnvalue (Class|ShooterGameMode|GetFloatOptionIni _asshootergamemode "SauropodPack" "AmpeloDamage"))
      (if (<= (Math|Float|Floor _returnvalue) 0)
        (Variables|Default|SetExtraReceiveDamageMultiplier 0.6)
        (else
          (Variables|Default|SetExtraReceiveDamageMultiplier _returnvalue))))))

(fn ConstructionScript
  (|CallParentFunction))

(fn GetExtraRunSpeedModifierPercent
  (bind _scaleextrarunningspeedmodifiermin (Variables|Default|GetScaleExtraRunningSpeedModifierMin))
  (if (== (Variables|Default|GetRider) 0)
    _
    (else
      (LocalVariables|SetPercentOut (/ (- (CallFunction|GetBestExtraRunSpeedModifier) _scaleextrarunningspeedmodifiermin) (- (Variables|Default|GetScaleExtraRunningSpeedModifierMax) _scaleextrarunningspeedmodifiermin)))))
  (return (LocalVariables|GetPercentOut)))

(fn GetBestExtraRunSpeedModifier
  (if (< (Math|Conversions|ToFloat(Integer) (- (Utilities|Time|GetGameTimeinSeconds) (Variables|Default|GetLastHigherScaleExtraRunningSpeedTime))) 0.55)
    (LocalVariables|SetretVal (Variables|Default|GetLastHigherScaleExtraRunningSpeedValue))
    (else
      (LocalVariables|SetretVal (Variables|Default|GetExtraRunningSpeedModifier))))
  (return (LocalVariables|GetretVal)))

(fn BPGetExtraMeleeDamageModifier
  (bind _newparam (CallFunction|GetExtraRunSpeedModifierPercent))
  (return (+ 1.0 (* (Variables|Default|GetMaxExtraSpeedAdditionalDamagePercent) _newparam))))

(fn BPGetHUDOverrideBuffProgressBarPercent
  (bind _newparam (CallFunction|GetExtraRunSpeedModifierPercent))
  (return _newparam))

(fn BPAdjustDamage
  (params (IncomingDamage :type Float%20%28single-precision%29) (TheDamageEvent :type Damage%20Event%20Structure) (EventInstigator :type Controller%20Object%20Reference) (DamageCauser :type Actor%20Object%20Reference) (bIsPointDamage :type Boolean) (PointHitInfo :type Hit%20Result%20Structure))
  (bind _mycharacterstatuscomponent (Variables|Default|GetMyCharacterStatusComponent))
  (Utilities|FlowControl|Sequence
    (:then_0
      (if bIsPointDamage
        (if (>= (Utilities|Array|FindItem (Variables|Default|GetTorporHeadBoneNames) (.HitBoneName (Collision|BreakHitResult PointHitInfo))) 0)
          (bind _returnvalue (Class|VictoryCore|GetClassDefaultObject (.DamageTypeClass (Utilities|Struct|BreakDamageEvent TheDamageEvent))))
          (bind _asshooterdamagetypebp_base_c (Utilities|Casting|CastToShooterDamageTypeBP_Base _returnvalue))
          (if (and (Variables|/Game/PrimalEarth/CoreBlueprints/DamageTypes/ShooterDamageTypeBP_Base.ShooterDamageTypeBP_Base_C|GetbCauseRaidTorpor _asshooterdamagetypebp_base_c) (Utilities|Enum|Equal(Enum) (Variables|/Script/Engine.CharacterMovementComponent|GetMovementMode (Variables|Character|GetCharacterMovement)) "MOVE_Walking"))
            (bind _asdinocharacterstatuscomponent_bp_torpiditycontrol_c (Utilities|Casting|CastToDinoCharacterStatusComponent_BP_TorpidityControl _mycharacterstatuscomponent))
            (Variables|/Game/PrimalEarth/CoreBlueprints/DinoCharacterStatusComponent_BP_TorpidityControl.DinoCharacterStatusComponent_BP_TorpidityControl_C|SetbAllowTorpidityIncrease _asdinocharacterstatuscomponent_bp_torpiditycontrol_c true)
            (Class|PrimalCharacterStatusComponent|ModifyCurrentStatusValue _mycharacterstatuscomponent "Torpidity" (* (Variables|/Game/PrimalEarth/CoreBlueprints/DamageTypes/ShooterDamageTypeBP_Base.ShooterDamageTypeBP_Base_C|GetRaidTorporDamageMultiplier _asshooterdamagetypebp_base_c) IncomingDamage (Variables|Default|GetTorporDamageMultiplier)) false false true false "/Script/Engine.DamageType" false false)
            (Variables|/Game/PrimalEarth/CoreBlueprints/DinoCharacterStatusComponent_BP_TorpidityControl.DinoCharacterStatusComponent_BP_TorpidityControl_C|SetbAllowTorpidityIncrease _asdinocharacterstatuscomponent_bp_torpiditycontrol_c false)
            (Variables|Default|SetbWildAllowTargetingNeutralStructures true)
            (Utilities|Time|SetTimerbyFunctionName 0 "TorporHit" 0.5)
            (Utilities|Time|SetTimerbyFunctionName 0 "ClearTorporHit" 6e+01)))))
    (:then_1
      (return IncomingDamage))))